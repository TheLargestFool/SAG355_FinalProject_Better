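; Demo actor for the aurora material that varies the animation timing of five line components, Line1 through Line5.
; The construction script gives each component a dynamic material instance built from Line1's material, then sets its time_offset parameter to a random value.
; Line1 is processed last, so the other lines copy its material before it receives its own instance.
; The event graph has no active logic.
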(event `self.ReceiveBeginPlay`)

(fn `UserConstructionScript`
  (bind _returnvalue (`KismetMathLibrary.RandomFloatInRange` 0.0 100.0))
  (bind _line_5 (`self.line_5`))
  (bind _line_4 (`self.line_4`))
  (bind _line_3 (`self.line_3`))
  (bind _line_2 (`self.line_2`))
  (bind _line_1 (`self.line_1`))
  (bind _returnvalue_2 (`PrimitiveComponent.GetMaterial` (`self.line_1`) 0))
  (`PrimitiveComponent.CreateDynamicMaterialInstance` _line_5 0 _returnvalue_2 "None")
  (`MeshComponent.SetScalarParameterValueOnMaterials` _line_5 "time_offset" _returnvalue)
  (`PrimitiveComponent.CreateDynamicMaterialInstance` _line_4 0 _returnvalue_2 "None")
  (`MeshComponent.SetScalarParameterValueOnMaterials` _line_4 "time_offset" _returnvalue)
  (`PrimitiveComponent.CreateDynamicMaterialInstance` _line_3 0 _returnvalue_2 "None")
  (`MeshComponent.SetScalarParameterValueOnMaterials` _line_3 "time_offset" _returnvalue)
  (`PrimitiveComponent.CreateDynamicMaterialInstance` _line_2 0 _returnvalue_2 "None")
  (`MeshComponent.SetScalarParameterValueOnMaterials` _line_2 "time_offset" _returnvalue)
  (`PrimitiveComponent.CreateDynamicMaterialInstance` _line_1 0 _returnvalue_2 "None")
  (`MeshComponent.SetScalarParameterValueOnMaterials` _line_1 "time_offset" _returnvalue))